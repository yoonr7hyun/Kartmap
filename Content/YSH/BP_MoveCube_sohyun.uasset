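; BP_MoveCube_sohyun is a player-controlled pawn that moves and turns through input axes.
; MoveForward adds movement input along the Camera's forward vector, scaled by the axis value.
; MoveRight and Turn both feed controller yaw, so MoveRight rotates the view instead of strafing.
; A camera right-vector movement node is left unconnected, and BeginPlay, overlap, Tick and the construction script are empty.
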(event EventBeginPlay)

(event Collision|EventActorBeginOverlap
  (params (OtherActor :type Actor%20Object%20Reference)))

(event EventTick
  (params (DeltaSeconds :type Float%20%28single-precision%29)))

(event Input|AxisEvents|InputAxisMoveForward
  (params (AxisValue :type Float%20%28single-precision%29))
  ;[1 1 1] Movenemt Input
  (Pawn|Input|AddMovementInput (* (Math|Vector|GetForwardVector (Variables|Default|GetCamera)) AxisValue) 1.0 false))

(event Input|AxisEvents|InputAxisMoveRight
  (params (AxisValue :type Float%20%28single-precision%29))
  ;[1 1 1] Movenemt Input
  (Pawn|Input|AddControllerYawInput AxisValue))

(event Input|AxisEvents|InputAxisTurn
  (params (AxisValue :type Float%20%28single-precision%29))
  (Pawn|Input|AddControllerYawInput AxisValue))

(fn ConstructionScript)