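; Chaos wheeled vehicle pawn that is driven each tick from axis inputs and prints its forward speed in MPH on screen.
; Throttle, brake and handbrake pass straight to the movement component.
; Horizontal look input builds a clamped steering angle that eases back to center faster at higher speed.
; While moving forward, the spring arm pitches, swings with steering and shifts back with speed; otherwise look input rotates it freely.
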(event EventTick
  (params (DeltaSeconds :type Float%20%28single-precision%29))
  (CallFunction|VehicleInputs)
  (CallFunction|CameraInput)
  (Development|PrintString (Utilities|String|Append (Utilities|String|ToString(Integer) (Math|Float|Round (Class|ChaosVehicleMovementComponent|GetForwardSpeedMPH (Variables|Default|GetVehicle_Component)))) "MPH") true true "(R=0.489583,G=0.034890,B=0.000000,A=1.000000)" 0.0))

(event EventBeginPlay
  (bind _aschaos_wheeled_vehicle_movement_component (Utilities|Casting|CastToChaosWheeledVehicleMovementComponent (Variables|Default|GetVehicleMovementComponent)))
  (Variables|Default|SetVehicle_Component _aschaos_wheeled_vehicle_movement_component))

(fn ConstructionScript)

(fn VehicleInputs
  (bind _vehiclemovementcomponent (Variables|Default|GetVehicleMovementComponent))
  (Class|ChaosVehicleMovementComponent|SetThrottleInput _vehiclemovementcomponent (Input|AxisValues|GetThrottle_Input))
  (Class|ChaosVehicleMovementComponent|SetBrakeInput _vehiclemovementcomponent (Input|AxisValues|GetBrake_Input))
  (Class|ChaosVehicleMovementComponent|SetHandbrakeInput _vehiclemovementcomponent (== (Input|AxisValues|GetHandbrake_Input) 1.0))
  (Variables|Default|SetStering_Angle (Math|Interpolation|FInterpTo (Math|Float|Clamp(Float) (+ (Variables|Default|GetStering_Angle) (* (Input|AxisValues|GetLookRight) 0.5)) -5e+01 5e+01) 0.0 (Utilities|Time|GetWorldDeltaSeconds) (Math|Float|MapRangeClamped (Class|ChaosVehicleMovementComponent|GetForwardSpeedMPH (Variables|Default|GetVehicle_Component)) 2e+01 75.0 3.0 15.0)))
  (Class|ChaosVehicleMovementComponent|SetSteeringInput _vehiclemovementcomponent (.yaw (Math|Rotator|Delta(Rotator) (Math|Rotator|MakeRotator 0.0 0.0 (* (Math|Interpolation|FInterpTo (Math|Float|Clamp(Float) (+ (Variables|Default|GetStering_Angle) (* (Input|AxisValues|GetLookRight) 0.5)) -5e+01 5e+01) 0.0 (Utilities|Time|GetWorldDeltaSeconds) (Math|Float|MapRangeClamped (Class|ChaosVehicleMovementComponent|GetForwardSpeedMPH (Variables|Default|GetVehicle_Component)) 2e+01 75.0 3.0 15.0)) 0.7)) (Math|Rotator|MakeRotator 0.0 0.0 0.0)))))

(fn CameraInput
  (bind _vehicle_component (Variables|Default|GetVehicle_Component))
  (bind _springarm (Variables|Default|GetSpringArm))
  (bind _returnvalue (Class|ChaosVehicleMovementComponent|GetForwardSpeedMPH _vehicle_component))
  (if (> _returnvalue 0.5)
    (Transformation|SetRelativeRotation _springarm (Math|Interpolation|RInterpTo (Variables|/Script/Engine.SceneComponent|GetRelativeRotation _springarm) (Math|Rotator|MakeRotator 0.0 (Math|Float|MapRangeClamped _returnvalue 0.0 7e+01 -6.0 -2e+01) (* (Variables|Default|GetStering_Angle) (Math|Float|MapRangeClamped _returnvalue 0.0 7e+01 2.0 1e+01))) (Utilities|Time|GetWorldDeltaSeconds) 3.0) false false)
    (Transformation|SetRelativeLocation (Variables|Default|GetSpringArm) (Math|Vector|MakeVector (Math|Float|MapRangeClamped _returnvalue 1.0 7e+01 -0.5 -3.5e+02) 0.0 85.0) false false)
    (else
      (Transformation|AddRelativeRotation (Variables|Default|GetSpringArm) (Math|Rotator|MakeRotator 0.0 (Input|AxisValues|GetLookUp) (Input|AxisValues|GetLookRight)) false false))))