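; BP_Car1 is a drivable Chaos wheeled vehicle Blueprint with a player-controlled spring arm camera.
; Every Tick it feeds throttle, brake and handbrake axes to the movement component and rotates the spring arm from look input.
; Steering derives from a clamped angle eased toward zero at a speed-dependent rate.
; Look-right is multiplied by zero in that calculation, so it turns only the camera, not the wheels.
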(event EventTick
  (params (DeltaSeconds :type Float%20%28single-precision%29))
  (CallFunction|VehicleInputs)
  (CallFunction|CameraInput))

(event EventBeginPlay
  (bind _aschaos_wheeled_vehicle_movement_component (Utilities|Casting|CastToChaosWheeledVehicleMovementComponent (Variables|Default|GetVehicleMovementComponent)))
  (Variables|Default|SetVehicle_Component _aschaos_wheeled_vehicle_movement_component))

(fn ConstructionScript)

(fn VehicleInputs
  (bind _vehiclemovementcomponent (Variables|Default|GetVehicleMovementComponent))
  (Class|ChaosVehicleMovementComponent|SetThrottleInput _vehiclemovementcomponent (Input|AxisValues|GetThrottle_Input))
  (Class|ChaosVehicleMovementComponent|SetBrakeInput _vehiclemovementcomponent (Input|AxisValues|GetBrake_Input))
  (Class|ChaosVehicleMovementComponent|SetHandbrakeInput _vehiclemovementcomponent (== (Input|AxisValues|GetHandbrake_Input) 1.0))
  (Variables|Default|SetStering_Angle (Math|Interpolation|FInterpTo (Math|Float|Clamp(Float) (+ (Variables|Default|GetStering_Angle) (* (Input|AxisValues|GetLookRight) 0.0)) -5e+01 5e+01) 0.0 (Utilities|Time|GetWorldDeltaSeconds) (Math|Float|MapRangeClamped (Class|ChaosVehicleMovementComponent|GetForwardSpeedMPH (Variables|Default|GetVehicle_Component)) 2e+01 75.0 3.0 15.0)))
  (Class|ChaosVehicleMovementComponent|SetSteeringInput _vehiclemovementcomponent (.yaw (Math|Rotator|Delta(Rotator) (Math|Rotator|MakeRotator 0.0 0.0 (* (Math|Interpolation|FInterpTo (Math|Float|Clamp(Float) (+ (Variables|Default|GetStering_Angle) (* (Input|AxisValues|GetLookRight) 0.0)) -5e+01 5e+01) 0.0 (Utilities|Time|GetWorldDeltaSeconds) (Math|Float|MapRangeClamped (Class|ChaosVehicleMovementComponent|GetForwardSpeedMPH (Variables|Default|GetVehicle_Component)) 2e+01 75.0 3.0 15.0)) 0.7)) (Math|Rotator|MakeRotator 0.0 0.0 0.0)))))

(fn CameraInput
  (Transformation|AddRelativeRotation (Variables|Default|GetSpringArm) (Math|Rotator|MakeRotator 0.0 (Input|AxisValues|GetLookUp) (Input|AxisValues|GetLookRight)) false false))