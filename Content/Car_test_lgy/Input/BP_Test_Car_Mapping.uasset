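; Test vehicle Blueprint that maps Enhanced Input actions to driving controls.
; On BeginPlay it adds the LGY_InputMapping context to the player controller's Enhanced Input subsystem.
; Throttle and brake actions feed their matching VehicleMovementComponent inputs, while the left and right "Detect Skidding" actions both set steering.
; Each action passes its value on both Triggered and Completed, so releases also update the vehicle.
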(event Input|EnhancedActionEvents|EnhancedInputActionIA_VH_LGY_Throttle
  (params (ActionValue :type Float%20%28double-precision%29) (ElapsedSeconds :type Float%20%28double-precision%29) (TriggeredSeconds :type Float%20%28double-precision%29) (InputAction :type Input%20Action%20Object%20Reference :default "/Game/Car_test_lgy/Input/IA_VH_LGY_Throttle.IA_VH_LGY_Throttle"))
  (:Triggered
    (Class|ChaosVehicleMovementComponent|SetThrottleInput (Variables|Default|GetVehicleMovementComponent) ActionValue :!label _label))
  (:Completed
    (goto _label)))

(event Input|EnhancedActionEvents|EnhancedInputActionIA_VH_LGY_Brake
  (params (ActionValue :type Float%20%28double-precision%29) (ElapsedSeconds :type Float%20%28double-precision%29) (TriggeredSeconds :type Float%20%28double-precision%29) (InputAction :type Input%20Action%20Object%20Reference :default "/Game/Car_test_lgy/Input/IA_VH_LGY_Brake.IA_VH_LGY_Brake"))
  (:Triggered
    (Class|ChaosVehicleMovementComponent|SetBrakeInput (Variables|Default|GetVehicleMovementComponent) ActionValue :!label _label))
  (:Completed
    (goto _label)))

(event Input|EnhancedActionEvents|EnhancedInputActionIA_VH_LGY_Steering
  (params (ActionValue :type Float%20%28double-precision%29) (ElapsedSeconds :type Float%20%28double-precision%29) (TriggeredSeconds :type Float%20%28double-precision%29) (InputAction :type Input%20Action%20Object%20Reference :default "/Game/Car_test_lgy/Input/IA_VH_LGY_Steering.IA_VH_LGY_Steering")))

(event Input|EnhancedActionEvents|EnhancedInputActionIA_Vehicle_Detect_Left_Skidding
  (params (ActionValue :type Float%20%28double-precision%29) (ElapsedSeconds :type Float%20%28double-precision%29) (TriggeredSeconds :type Float%20%28double-precision%29) (InputAction :type Input%20Action%20Object%20Reference :default "/Game/Car_test_lgy/Input/IA_Vehicle_Detect_Left_Skidding.IA_Vehicle_Detect_Left_Skidding"))
  (:Triggered
    (Class|ChaosVehicleMovementComponent|SetSteeringInput (Variables|Default|GetVehicleMovementComponent) ActionValue :!label _label))
  (:Completed
    (goto _label)))

(event Input|EnhancedActionEvents|EnhancedInputActionIA_Vehicle_Detect_Right_Skidding
  (params (ActionValue :type Float%20%28double-precision%29) (ElapsedSeconds :type Float%20%28double-precision%29) (TriggeredSeconds :type Float%20%28double-precision%29) (InputAction :type Input%20Action%20Object%20Reference :default "/Game/Car_test_lgy/Input/IA_Vehicle_Detect_Right_Skidding.IA_Vehicle_Detect_Right_Skidding"))
  (:Triggered
    (Class|ChaosVehicleMovementComponent|SetSteeringInput (Variables|Default|GetVehicleMovementComponent) ActionValue :!label _label))
  (:Completed
    (goto _label)))

(event EventBeginPlay
  ;[1 1 1] 키 맵핑
  (bind _as플레이어_컨트롤러 (Utilities|Casting|CastToPlayerController (Pawn|GetController)))
  (Utilities|IsValid (PlayerController|LocalPlayerSubsystems|GetEnhancedInputLocalPlayerSubsystem _as플레이어_컨트롤러)
    (:Is%20Valid
      (Input|AddMappingContext (PlayerController|LocalPlayerSubsystems|GetEnhancedInputLocalPlayerSubsystem _as플레이어_컨트롤러) "/Game/Car_test_lgy/Input/LGY_InputMapping.LGY_InputMapping" 0 "(bIgnoreAllPressedKeysUntilRelease=True,bForceImmediately=False)"))))

(fn ConstructionScript)