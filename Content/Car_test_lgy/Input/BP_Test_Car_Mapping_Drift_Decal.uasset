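; Test Chaos wheeled-vehicle pawn that adds drift skid decals and VFX to a drivable car.
; Enhanced Input actions feed throttle, brake, steering and handbrake into the movement component.
; Tick damps airborne rotation, recenters the spring-arm yaw, and flags drift purely by forward speed.
; While drifting, holding a hard-coded Left Shift spawns decals every frame at two arrows; pressing it activates two VFX, cleared on release or low speed.
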(event Custom|InterpsToOriginalRotation
  ;[1 1 1] 데칼
  (Transformation|SetRelativeRotation (Variables|Default|GetSpringArm) (Math|Rotator|MakeRotator 0.0 0.0 (Math|Interpolation|FInterpTo (.yaw (Variables|/Script/Engine.SceneComponent|GetRelativeRotation (Variables|Default|GetSpringArm))) 0.0 (Utilities|Time|GetWorldDeltaSeconds) 1.0)) false false) ; Reset camera to original angle
)

(event Input|EnhancedActionEvents|EnhancedInputActionIA_Vehicle_Move_FWD
  (params (ActionValue :type Float%20%28double-precision%29) (ElapsedSeconds :type Float%20%28double-precision%29) (TriggeredSeconds :type Float%20%28double-precision%29) (InputAction :type Input%20Action%20Object%20Reference :default "/Game/Car_test_lgy/Input/IA_Vehicle_Move_FWD.IA_Vehicle_Move_FWD"))
  (bind _chaoswheeledvehiclemovement (Variables|Default|GetChaosWheeledVehicleMovement))
  ;[1 1 1] 무브먼트
  (:Triggered
    (Class|ChaosVehicleMovementComponent|SetThrottleInput _chaoswheeledvehiclemovement ActionValue :!label _label)
    (Development|PrintString (Utilities|String|Append (Utilities|String|ToString(Integer) (Math|Float|Round (Class|ChaosVehicleMovementComponent|GetForwardSpeedMPH _chaoswheeledvehiclemovement))) "go") true true "(R=0.000000,G=0.660000,B=1.000000,A=1.000000)" 0.0))
  (:Completed
    (goto _label)))

(event Input|EnhancedActionEvents|EnhancedInputActionIA_Vehicle_Move_BWD
  (params (ActionValue :type Float%20%28double-precision%29) (ElapsedSeconds :type Float%20%28double-precision%29) (TriggeredSeconds :type Float%20%28double-precision%29) (InputAction :type Input%20Action%20Object%20Reference :default "/Game/Car_test_lgy/Input/IA_Vehicle_Move_BWD.IA_Vehicle_Move_BWD"))
  ;[1 1 1] 무브먼트
  (:Triggered
    (Class|ChaosVehicleMovementComponent|SetBrakeInput (Variables|Default|GetChaosWheeledVehicleMovement) ActionValue :!label _label))
  (:Completed
    (goto _label)))

(event Input|EnhancedActionEvents|EnhancedInputActionIA_Vehicle_Move_Steering
  (params (ActionValue :type Float%20%28double-precision%29) (ElapsedSeconds :type Float%20%28double-precision%29) (TriggeredSeconds :type Float%20%28double-precision%29) (InputAction :type Input%20Action%20Object%20Reference :default "/Game/Car_test_lgy/Input/IA_Vehicle_Move_Steering.IA_Vehicle_Move_Steering"))
  ;[1 1 1] 무브먼트
  (:Triggered
    (Class|ChaosVehicleMovementComponent|SetSteeringInput (Variables|Default|GetChaosWheeledVehicleMovement) ActionValue :!label _label))
  (:Completed
    (goto _label)))

(event Input|EnhancedActionEvents|EnhancedInputActionIA_Vehicle_Brake
  (params (ActionValue :type Float%20%28double-precision%29) (ElapsedSeconds :type Float%20%28double-precision%29) (TriggeredSeconds :type Float%20%28double-precision%29) (InputAction :type Input%20Action%20Object%20Reference :default "/Game/Car_test_lgy/Input/IA_Vehicle_Brake.IA_Vehicle_Brake"))
  (bind _chaoswheeledvehiclemovement (Variables|Default|GetChaosWheeledVehicleMovement))
  ;[1 1 1] 드리프트 테스트
  (:Triggered
    (Class|ChaosVehicleMovementComponent|SetHandbrakeInput _chaoswheeledvehiclemovement (== ActionValue 1.0) :!label _label)
    (if (> (.SkidMagnitude (Class|ChaosWheeledVehicleMovementComponent|BreakWheelStatus _chaoswheeledvehiclemovement (Class|ChaosWheeledVehicleMovementComponent|GetWheelState (Variables|Default|GetChaosWheeledVehicleMovement) 3))) -1e+01)
      (Utilities|FlowControl|Delay 3e+01)
      (Development|PrintString (Utilities|String|Append (Utilities|String|ToString(Integer) (Math|Float|Round (Class|ChaosVehicleMovementComponent|GetForwardSpeedMPH (Variables|Default|GetChaosWheeledVehicleMovement)))) "Drift") true true "(R=0.000000,G=0.660000,B=1.000000,A=1.000000)" 0.0)
      (else
        (Utilities|FlowControl|Delay 0.5))))
  (:Completed
    (goto _label)))

(event EventTick
  (params (DeltaSeconds :type Float%20%28single-precision%29))
  (bind _vehiclemovementcomponent (Variables|Default|GetVehicleMovementComponent))
  (bind _relative_transform_scale_x (Variables|디폴트|GetRelative%20Transform%20Scale%20X))
  (bind _arrow (Variables|Default|GetArrow))
  (bind _arrow1 (Variables|Default|GetArrow1))
  (bind _returnvalue (Vehicle|GetForwardSpeed _vehiclemovementcomponent))
  (bind _returnvalue_2 (Transformation|GetWorldTransform _arrow1))
  (bind _returnvalue_3 (Transformation|GetWorldTransform _arrow))
  (bind (_location _rotation) (Math|Transform|BreakTransform _returnvalue_2))
  (bind (_location_2 _rotation_2) (Math|Transform|BreakTransform _returnvalue_3))
  ;[1 1 1] 데칼
  (Class|PrimitiveComponent|SetAngularDamping (Variables|Character|GetMesh) (Math|Float|SelectFloat 0.0 3.0 (AI|Components|NavMovement|IsMovingonGround (Variables|Default|GetChaosWheeledVehicleMovement)))) ; Damps rotation when in air
  (CallFunction|InterpstoOriginalRotation)
  (Utilities|FlowControl|Sequence
    (:then_0
      (if (<= _returnvalue 5e+02)
        (Components|Activation|SetActive (Variables|Default|GetVFX_Drift) false false)))
    (:then_1
      (if (>= _returnvalue 1e+03)
        (Variables|디폴트|SetDrift true)
        (if (and (Variables|디폴트|GetDrift) (Variables|Default|GetBrak%20Pressing%20))
          (AddComponent|AddDecalComponent true (Math|Transform|MakeTransform _location_2 _rotation_2 (Math|Vector|MakeVector _relative_transform_scale_x _relative_transform_scale_x _relative_transform_scale_x)))
          (AddComponent|AddDecalComponent true (Math|Transform|MakeTransform _location _rotation (Math|Vector|MakeVector _relative_transform_scale_x _relative_transform_scale_x _relative_transform_scale_x))))
        (else
          (Variables|디폴트|SetDrift false))))))

(event EventBeginPlay
  ;[1 1 1] 키 맵핑
  (CallFunction|KeymappingInputs))

(event Input|KeyboardEvents|LeftShift
  (params (Key :type Key%20Structure :default "None"))
  (bind _vfx_drift (Variables|Default|GetVFX_Drift))
  ;[1 1 1] 데칼
  (:Pressed
    (Variables|Default|SetBrak%20Pressing%20 true)
    (if (Variables|디폴트|GetDrift)
      (Components|Activation|SetActive _vfx_drift true false)))
  (:Released
    (Variables|Default|SetBrak%20Pressing%20 false)
    (Components|Activation|SetActive _vfx_drift false false)))

(fn ConstructionScript)

(fn VehicleInputs
  (bind _chaoswheeledvehiclemovement (Variables|Default|GetChaosWheeledVehicleMovement))
  (Class|ChaosVehicleMovementComponent|SetThrottleInput _chaoswheeledvehiclemovement (Input|EnhancedActionValues|GetIA_Vehicle_Move_FWD))
  (Class|ChaosVehicleMovementComponent|SetBrakeInput _chaoswheeledvehiclemovement (Input|EnhancedActionValues|GetIA_Vehicle_Move_BWD))
  (Class|ChaosVehicleMovementComponent|SetSteeringInput _chaoswheeledvehiclemovement (Input|EnhancedActionValues|GetIA_Vehicle_Move_Steering))
  (Class|ChaosVehicleMovementComponent|SetHandbrakeInput _chaoswheeledvehiclemovement (== (Input|EnhancedActionValues|GetIA_Vehicle_Brake) 1.0)))

(fn KeymappingInputs
  ;[1 1 1] 키 맵핑 연결
  (bind _as플레이어_컨트롤러 (Utilities|Casting|CastToPlayerController (Pawn|GetController)))
  (Utilities|IsValid (PlayerController|LocalPlayerSubsystems|GetEnhancedInputLocalPlayerSubsystem _as플레이어_컨트롤러)
    (:Is%20Valid
      (Input|AddMappingContext (PlayerController|LocalPlayerSubsystems|GetEnhancedInputLocalPlayerSubsystem _as플레이어_컨트롤러) "/Game/Car_test_lgy/Input/LGY_InputMapping.LGY_InputMapping" 0 "(bIgnoreAllPressedKeysUntilRelease=True,bForceImmediately=False)"))))

(fn CameraRotate
  (params (self2 :type Chaos%20Vehicle%20Movement%20Component%20Object%20Reference))
  (Variables|Default|SetStering%20Angle (Math|Interpolation|FInterpTo (Math|Float|Clamp(Float) (+ (Variables|Default|GetStering%20Angle) (+ (Input|AxisValues|GetLookRight) 0.5)) -1e+01 1e+01) 0.0 (Utilities|Time|GetWorldDeltaSeconds) (Math|Float|MapRangeClamped (Class|ChaosVehicleMovementComponent|GetForwardSpeedMPH (Variables|Default|GetChaosWheeledVehicleMovement)) 2e+01 75.0 3.0 15.0)))
  (Class|ChaosVehicleMovementComponent|SetSteeringInput self2 (.yaw (Math|Rotator|Delta(Rotator) (Math|Rotator|MakeRotator 0.0 0.0 (* (Math|Interpolation|FInterpTo (Math|Float|Clamp(Float) (+ (Variables|Default|GetStering%20Angle) (+ (Input|AxisValues|GetLookRight) 0.5)) -1e+01 1e+01) 0.0 (Utilities|Time|GetWorldDeltaSeconds) (Math|Float|MapRangeClamped (Class|ChaosVehicleMovementComponent|GetForwardSpeedMPH (Variables|Default|GetChaosWheeledVehicleMovement)) 2e+01 75.0 3.0 15.0)) 0.7)) (Math|Rotator|MakeRotator 0.0 0.0 0.0)))))